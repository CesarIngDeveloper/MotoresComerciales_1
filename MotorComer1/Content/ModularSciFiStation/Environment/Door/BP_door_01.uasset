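; Automatic sci-fi station door that opens when anything overlaps its Box trigger and closes after it leaves.
; Overlap plays the Door timeline, whose separate tracks lerp the relative locations of seven panels: bottom and side pairs slide apart sideways, three middle panels rise.
; End overlap waits one second, then reverses the same timeline to close, with no check on which actor triggered it or whether others remain inside.
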(event OnComponentBeginOverlap(Box)
  (params (OverlappedComponent :type Primitive%20Component%20Object%20Reference) (OtherActor :type Actor%20Object%20Reference) (OtherComp :type Primitive%20Component%20Object%20Reference) (OtherBodyIndex :type Integer) (bFromSweep :type Boolean) (SweepResult :type Hit%20Result%20Structure%20%28by%20ref%29))
  (bind (_direction _top1_door _top2_door _top3_door _side_door _bot_door) (Timeline|door Play)
    (:Update
      (Utilities|FlowControl|Sequence
        (:then_0
          (Transformation|SetRelativeLocation (Variables|Default|Getdoor_bot_left) (Math|Vector|Lerp(Vector) "0, 0, 0" "0,50.000000, 0" _bot_door) false false))
        (:then_1
          (Transformation|SetRelativeLocation (Variables|Default|Getdoor_bot_right) (Math|Vector|Lerp(Vector) "0, 0, 0" "0,-50.000000, 0" _bot_door) false false))
        (:then_2
          (Transformation|SetRelativeLocation (Variables|Default|Getdoor_mid_01) (Math|Vector|Lerp(Vector) "0, 0, 0" "0,0.000000,50.000000" _top1_door) false false))
        (:then_3
          (Transformation|SetRelativeLocation (Variables|Default|Getdoor_mid_02) (Math|Vector|Lerp(Vector) "0, 0, 0" "0,0.000000,60.000000" _top2_door) false false))
        (:then_4
          (Transformation|SetRelativeLocation (Variables|Default|Getdoor_mid_03) (Math|Vector|Lerp(Vector) "0, 0, 0" "0,0.000000,65.000000" _top3_door) false false))
        (:then_5
          (Transformation|SetRelativeLocation (Variables|Default|Getdoor_right) (Math|Vector|Lerp(Vector) "0, 0, 0" "0,-50.000000, 0" _side_door) false false))
        (:then_6
          (Transformation|SetRelativeLocation (Variables|Default|Getdoor_left) (Math|Vector|Lerp(Vector) "0, 0, 0" "0,50.000000, 0" _side_door) false false))))))

(event OnComponentEndOverlap(Box)
  (params (OverlappedComponent :type Primitive%20Component%20Object%20Reference) (OtherActor :type Actor%20Object%20Reference) (OtherComp :type Primitive%20Component%20Object%20Reference) (OtherBodyIndex :type Integer))
  (Utilities|FlowControl|Delay 1.0)
  (bind (_direction _top1_door _top2_door _top3_door _side_door _bot_door) (Timeline|door Reverse)
    (:Update
      (Utilities|FlowControl|Sequence
        (:then_0
          (Transformation|SetRelativeLocation (Variables|Default|Getdoor_bot_left) (Math|Vector|Lerp(Vector) "0, 0, 0" "0,50.000000, 0" _bot_door) false false))
        (:then_1
          (Transformation|SetRelativeLocation (Variables|Default|Getdoor_bot_right) (Math|Vector|Lerp(Vector) "0, 0, 0" "0,-50.000000, 0" _bot_door) false false))
        (:then_2
          (Transformation|SetRelativeLocation (Variables|Default|Getdoor_mid_01) (Math|Vector|Lerp(Vector) "0, 0, 0" "0,0.000000,50.000000" _top1_door) false false))
        (:then_3
          (Transformation|SetRelativeLocation (Variables|Default|Getdoor_mid_02) (Math|Vector|Lerp(Vector) "0, 0, 0" "0,0.000000,60.000000" _top2_door) false false))
        (:then_4
          (Transformation|SetRelativeLocation (Variables|Default|Getdoor_mid_03) (Math|Vector|Lerp(Vector) "0, 0, 0" "0,0.000000,65.000000" _top3_door) false false))
        (:then_5
          (Transformation|SetRelativeLocation (Variables|Default|Getdoor_right) (Math|Vector|Lerp(Vector) "0, 0, 0" "0,-50.000000, 0" _side_door) false false))
        (:then_6
          (Transformation|SetRelativeLocation (Variables|Default|Getdoor_left) (Math|Vector|Lerp(Vector) "0, 0, 0" "0,50.000000, 0" _side_door) false false))))))

(fn ConstructionScript)